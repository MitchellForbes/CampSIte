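; BP_Camera is a camera Blueprint that performs a fixed yaw swing when its Rotate event is called.
; BeginPlay caches the actor's starting rotation and a target rotation offset 15 degrees in negative yaw.
; Rotate plays the Rotation timeline from the start, using its track as the alpha to lerp between the cached rotations.
; Because both endpoints are cached once, each call replays the same swing rather than accumulating.
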(event `self.ReceiveBeginPlay`
  (bind _returnvalue (`self.K2_GetActorRotation`))
  (set `self.NewVar` _returnvalue)
  (set `self.NewVar_0` (`KismetMathLibrary.MakeRotator` (.roll _returnvalue) (.pitch _returnvalue) (- (.yaw _returnvalue) 15.0))))

(event `Rotate`
  (bind (_direction _camera_rotation) (`Timeline|Rotation` :!via `PlayFromStart`)
    (:`Update`
      (`self.K2_SetActorRotation` (`KismetMathLibrary.RLerp` (`self.NewVar`) (`self.NewVar_0`) _camera_rotation)))))

(fn `UserConstructionScript`)